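; BP_Door_Anim is an animated door for the horror mansion that swings open and closed.
; A Box overlap sets DoorStatus, which gates the MainDoor_anim event so it only acts while something is inside the box.
; Each accepted call alternates through a FlipFlop between playing and reversing the Open_close timeline, whose OpenDoor track drives the Door's relative yaw.
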(event OnComponentBeginOverlap(Box)
  (params (OverlappedComponent :type Primitive%20Component%20Object%20Reference) (OtherActor :type Actor%20Object%20Reference) (OtherComp :type Primitive%20Component%20Object%20Reference) (OtherBodyIndex :type Integer) (bFromSweep :type Boolean) (SweepResult :type Hit%20Result%20Structure%20%28by%20ref%29))
  (Variables|Default|SetDoor_status true))

(event OnComponentEndOverlap(Box)
  (params (OverlappedComponent :type Primitive%20Component%20Object%20Reference) (OtherActor :type Actor%20Object%20Reference) (OtherComp :type Primitive%20Component%20Object%20Reference) (OtherBodyIndex :type Integer))
  (Variables|Default|SetDoor_status false))

(event Custom|MainDoor_anim
  (if (Variables|Default|GetDoor_status)
    (Utilities|FlowControl|FlipFlop
      (:A
        (bind _open_door (Timeline|Open_close Play)
          (:Update
            (Transformation|SetRelativeRotation (Variables|Default|GetDoor) (Math|Rotator|MakeRotator 0.0 0.0 _open_door) false false))))
      (:B
        (Timeline|Open_close Reverse)))))

(fn ConstructionScript)