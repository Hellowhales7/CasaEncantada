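; Interactable chair actor that moves the first-person player onto it and highlights while the player is nearby.
; The Box overlap events toggle custom depth rendering on the chair mesh when BP_FirstPerson enters or leaves.
; Interact teleports the player character to a point 100 units up in the chair's local space, using a location-only transform that does not carry over the chair's rotation.
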(event OnComponentBeginOverlap(Box)
  (params (OverlappedComponent :type Primitive%20Component%20Object%20Reference) (OtherActor :type Actor%20Object%20Reference) (OtherComp :type Primitive%20Component%20Object%20Reference) (OtherBodyIndex :type Integer) (bFromSweep :type Boolean) (SweepResult :type Hit%20Result%20Structure%20%28by%20ref%29))
  (Utilities|Casting|CastToBP_FirstPerson OtherActor)
  (Rendering|SetRenderCustomDepth (Variables|Default|GetSM_Chair) true))

(event OnComponentEndOverlap(Box)
  (params (OverlappedComponent :type Primitive%20Component%20Object%20Reference) (OtherActor :type Actor%20Object%20Reference) (OtherComp :type Primitive%20Component%20Object%20Reference) (OtherBodyIndex :type Integer))
  (Utilities|Casting|CastToBP_FirstPerson OtherActor)
  (Rendering|SetRenderCustomDepth (Variables|Default|GetSM_Chair) false))

(event EventBeginPlay)

(event Collision|EventActorBeginOverlap
  (params (OtherActor :type Actor%20Object%20Reference)))

(event EventTick
  (params (DeltaSeconds :type Float%20%28single-precision%29)))

(event EventInteract
  (bind _asbp_first_person (Utilities|Casting|CastToBP_FirstPerson (Game|GetPlayerCharacter 0)))
  (Transformation|SetActorTransform _asbp_first_person (Math|Conversions|ToTransform(Vector) (Math|Transform|TransformLocation (Transformation|GetActorTransform) "0.000000,0.000000,100.000000")) false true))

(fn ConstructionScript)