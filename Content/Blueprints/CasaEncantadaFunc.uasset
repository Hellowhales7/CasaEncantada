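; CasaEncantadaFunc is a shared function Blueprint whose Notice function shows an on-screen message to the player.
; Notice removes any top-level NoticeWB widgets, then creates a new one with front, bold and body text and adds it to the viewport, so each notice replaces the last.
; A disconnected check of the BP_FirstPerson Notification variable remains in the graph but never runs.
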(fn Notice
  (params (FrontMessage :type Text) (BoldMessage :type Text) (Message :type Text))
  (bind _foundwidgets (Widget|GetAllWidgetsOfClass 0 "/Game/UI/NoticeWB.NoticeWB_C"))
  (Widget|RemovefromParent _foundwidgets)
  (bind _returnvalue (UserInterface|CreateWidget "/Game/UI/NoticeWB.NoticeWB_C"))
  (Variables|/Game/UI/NoticeWB.NoticeWB_C|SetFrontMessageText _returnvalue FrontMessage)
  (Variables|/Game/UI/NoticeWB.NoticeWB_C|SetItemText _returnvalue BoldMessage)
  (Variables|/Game/UI/NoticeWB.NoticeWB_C|SetMessageText _returnvalue Message)
  (UserInterface|Viewport|AddtoViewport _returnvalue 1))