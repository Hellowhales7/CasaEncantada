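; Interactable drawer actor that slides a drawer open when its Interact event fires.
; Interact line-traces from the BP_FirstPerson camera for a WorldDynamic static mesh component, plays a sound and stores that mesh as the moving part.
; A timeline lerps the mesh 10 units along relative Y from its current location.
; No closing or limit is wired, so each interaction restarts the slide from the current position.
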(event EventBeginPlay
  (Input|EnableInput (Game|GetPlayerController 0)))

(event EventInteract
  (bind _asbp_first_person (Utilities|Casting|CastToBP_FirstPerson (Game|GetPlayerCharacter 0)))
  (bind (_outhit _returnvalue) (Collision|LineTraceForObjects (Transformation|GetWorldLocation (Variables|/Game/ThirdPerson/Blueprints/BP_FirstPerson.BP_FirstPerson_C|GetFollowCamera _asbp_first_person)) (+ (Transformation|GetWorldLocation (Variables|/Game/ThirdPerson/Blueprints/BP_FirstPerson.BP_FirstPerson_C|GetFollowCamera _asbp_first_person)) (* (Math|Vector|GetForwardVector (Variables|/Game/ThirdPerson/Blueprints/BP_FirstPerson.BP_FirstPerson_C|GetFollowCamera _asbp_first_person)) "500.000000,500.000000,500.000000")) (Utilities|Array|MakeArray "ObjectTypeQuery2") false 0 "ForDuration" false))
  (if _returnvalue
    (bind _as스태틱_메시_컴포넌트 (Utilities|Casting|CastToStaticMeshComponent (.HitComponent (Collision|BreakHitResult _outhit))))
    (Variables|Default|SetStatic%20Mesh%20REF _as스태틱_메시_컴포넌트)
    (Audio|PlaySoundatLocation 0 (Transformation|GetActorLocation) "0, 0, 0" 1.0 1.0 0.0 0 0 0 0)
    (Variables|Default|SetStartLoc (Math|Vector|MakeVector (.x (Variables|/Script/Engine.SceneComponent|GetRelativeLocation (Variables|Default|GetStatic%20Mesh%20REF))) (.y (Variables|/Script/Engine.SceneComponent|GetRelativeLocation (Variables|Default|GetStatic%20Mesh%20REF))) (.z (Variables|/Script/Engine.SceneComponent|GetRelativeLocation (Variables|Default|GetStatic%20Mesh%20REF)))))
    (Variables|Default|SetEndLoc (Math|Vector|MakeVector (.x (Variables|/Script/Engine.SceneComponent|GetRelativeLocation (Variables|Default|GetStatic%20Mesh%20REF))) (+ (.y (Variables|/Script/Engine.SceneComponent|GetRelativeLocation (Variables|Default|GetStatic%20Mesh%20REF))) 1e+01) (.z (Variables|/Script/Engine.SceneComponent|GetRelativeLocation (Variables|Default|GetStatic%20Mesh%20REF)))))
    (bind _새_트랙_0 (Timeline|타임라인 PlayFromStart)
      (:Update
        (Transformation|SetRelativeLocation (Variables|Default|GetStatic%20Mesh%20REF) (Math|Vector|Lerp(Vector) (Variables|Default|GetStartLoc) (Variables|Default|GetEndLoc) _새_트랙_0) false false)))))

(fn ConstructionScript)