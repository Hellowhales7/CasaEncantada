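; EmptyPot is an interactable pot where the first-person player plants a seed.
; Interact scans the player's slots for a Seed item, then spawns a Seed actor at a slight offset unless the PlayerState's Planting flag is already set.
; It sets that flag on planting and shows a notice, also warning for every non-seed slot.
; A sphere overlap toggles the cube's custom depth while the player is near.
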(event OnComponentBeginOverlap(Sphere)
  (params (OverlappedComponent :type Primitive%20Component%20Object%20Reference) (OtherActor :type Actor%20Object%20Reference) (OtherComp :type Primitive%20Component%20Object%20Reference) (OtherBodyIndex :type Integer) (bFromSweep :type Boolean) (SweepResult :type Hit%20Result%20Structure%20%28by%20ref%29))
  (Utilities|Casting|CastToBP_FirstPerson OtherActor)
  (Rendering|SetRenderCustomDepth (Variables|Default|GetCube) true))

(event OnComponentEndOverlap(Sphere)
  (params (OverlappedComponent :type Primitive%20Component%20Object%20Reference) (OtherActor :type Actor%20Object%20Reference) (OtherComp :type Primitive%20Component%20Object%20Reference) (OtherBodyIndex :type Integer))
  (Utilities|Casting|CastToBP_FirstPerson OtherActor)
  (Rendering|SetRenderCustomDepth (Variables|Default|GetCube) false))

(event EventInteract
  (bind _returnvalue (Transformation|GetActorTransform))
  (bind _asbp_first_person (Utilities|Casting|CastToBP_FirstPerson (Game|Player|GetPlayerPawn 0)))
  (for _array_element (Variables|/Game/ThirdPerson/Blueprints/BP_FirstPerson.BP_FirstPerson_C|GetPlayerSlot _asbp_first_person)
    (if (Utilities|Enum|Equal(Enum) (Utilities|String|ToString(Name) (.RowName (Utilities|Struct|BreakDataTableRowHandle (.Item (Utilities|Struct|BreakSlots _array_element))))) "Seed")
      (bind _asmy_player_state (Utilities|Casting|CastToMyPlayerState (Game|GetPlayerState 0)))
      (if (not (Variables|/Game/ThirdPerson/Blueprints/MyPlayerState.MyPlayerState_C|GetPlanting _asmy_player_state))
        (Variables|/Game/ThirdPerson/Blueprints/MyPlayerState.MyPlayerState_C|SetPlanting _asmy_player_state true)
        (Game|SpawnActorfromClass "/Game/Item/Seed.Seed_C" (Math|Transform|MakeTransform (+ (.location _returnvalue) "0.000000,10.000000,0.000000") (.rotation _returnvalue) (.scale _returnvalue)) "Undefined" 0 0)
        (CallFunction|Notice "Planted a seed."))
      (else
        (CallFunction|Notice "Need something to plant.")))))

(fn ConstructionScript)