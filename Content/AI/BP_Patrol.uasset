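; BP_Patrol is an AI patrol enemy that reacts to spotting the player through a PawnSensing component.
; When it sees a pawn tagged Player, it sets the seeingPlayer flag on its AI controller's blackboard.
; If no chase music instance is valid, it spawns and fades in the Chasing sound, then calls GameOver on the first-person player character.
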(event OnSeePawn(PawnSensing)
  (params (Pawn :type Pawn%20Object%20Reference))
  (if (Actor|ActorHasTag Pawn "Player")
    (AI|Components|Blackboard|SetValueasBool (AI|GetBlackboard (AI|GetAIController self)) (Utilities|Name|MakeLiteralName "seeingPlayer") true)
    (Variables|Default|GetChasingMusic
      (:then)
      (:else
        (bind _returnvalue (Audio|SpawnSound2D "/Game/Audio/Chasing.Chasing" 2.0 1.0 0.0 0))
        (bind _output_get (Variables|Default|SetChasingMusic _returnvalue))
        (Audio|Components|Audio|FadeIn _output_get 3.0 1.0 0.0 "Linear" :!class /Script/Engine.AudioComponent)
        (bind _asbp_first_person (Utilities|Casting|CastToBP_FirstPerson (Game|GetPlayerCharacter 0)))
        (Default|GameOver _asbp_first_person)))))

(event EventBeginPlay)

(fn ConstructionScript)